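; BP_ZombiePawn is an enemy zombie pawn that faces and chases the first player's pawn.
; BeginPlay caches the player and speed; Tick turns the actor toward the player and calls a custom movement event.
; That event applies an unswept, horizontally normalized offset toward the player, scaled by speed per frame without delta time.
; The detection-range comparison is unconnected and the branch is always true, so the chase has no distance limit.
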(event `self.ReceiveBeginPlay`
  (`|ExecutionSequence`
    (:`then_0`
      (set `self.Player` (`GameplayStatics.GetPlayerPawn` 0)))
    (:`then_1`
      (set `self.EnemySpeed` 10))))

(event `self.ReceiveTick`
  (params (DeltaSeconds :type "Float (single-precision)"))
  (`|ExecutionSequence`
    (:`then_0`
      (`self.K2_SetActorRotation` (`KismetMathLibrary.FindLookAtRotation` (`self.K2_GetActorLocation`) (`self.K2_GetActorLocation` (`self.Player`)))))
    (:`then_1`
      (`self.CustomEvent_1`))))

(event `CustomEvent_1`
  (bind _player (`self.Player`))
  (`/Engine/EditorBlueprintResources/StandardMacros.IsValid` _player
    (:`Is Valid`
      (set `self.Enemy Detection Range` 10)
      (if true
        (`self.K2_AddActorWorldOffset` (* (* (`KismetMathLibrary.Vector_Normal2D` (- (`self.K2_GetActorLocation`) (`self.K2_GetActorLocation` _player))) -1) (`self.EnemySpeed`)))))))

(fn `UserConstructionScript`)